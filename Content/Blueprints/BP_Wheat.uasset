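; BP_Wheat is a harvestable wheat crop that grows on a timer and is collected by clicking.
; On BeginPlay it waits a short delay, then switches its Sphere to a green material and sets IsGrown.
; Clicking the Sphere once grown adds one wheat through BP_GameInstance and destroys the actor.
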(event OnClicked(Sphere)
  (params (TouchedComponent :type Primitive%20Component%20Object%20Reference) (ButtonPressed :type Key%20Structure :default "None"))
  (if (Variables|Default|GetIsGrown?)
    (bind _asbp_game_instance (Utilities|Casting|CastToBP_GameInstance (Game|GetGameInstance)))
    (Default|AddWheat _asbp_game_instance 1)
    (Actor|DestroyActor)))

(event EventBeginPlay
  (Utilities|FlowControl|Delay 5.0)
  (Rendering|Material|SetMaterial (Variables|Default|GetSphere) 0 "/Game/Materials/M_Green.M_Green")
  (Variables|Default|SetIsGrown? true))

(event Collision|EventActorBeginOverlap
  (params (OtherActor :type Actor%20Object%20Reference)))

(event EventTick
  (params (DeltaSeconds :type Float%20%28single-precision%29)))

(fn ConstructionScript)