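; BP_Camera is a camera Blueprint that handles player input for pause and money changes, with no camera movement logic in its graphs.
; BeginPlay sets game-only input with a visible cursor.
; IA_PauseGame toggles WBP_PauseMenu, game pause and input mode, hiding the cursor on resume.
; Keys 1 and 2 add or remove money through BP_GameInstance, while a BP_ResourceManager lookup is left unconnected.
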(event Input|EnhancedActionEvents|EnhancedInputActionIA_PauseGame
  (params (ActionValue :type Boolean) (ElapsedSeconds :type Float%20%28double-precision%29) (TriggeredSeconds :type Float%20%28double-precision%29) (InputAction :type Input%20Action%20Object%20Reference :default "/Game/Input/Actions/IA_PauseGame.IA_PauseGame"))
  (if (not (Variables|Default|GetIsPauseMenuOpened?))
    (Variables|Default|SetIsPauseMenuOpened? true)
    (bind _returnvalue (UserInterface|CreateWidget "/Game/UI/WBP_PauseMenu.WBP_PauseMenu_C" (Game|GetPlayerController 0)))
    (bind _output_get (Variables|Default|SetPauseMenuWidget _returnvalue))
    (UserInterface|Viewport|AddtoViewport _output_get 0)
    (Input|SetInputModeGameandUI (Game|GetPlayerController 0) (Variables|Default|GetPauseMenuWidget) "DoNotLock" true false)
    (Variables|/Script/Engine.PlayerController|SetbShowMouseCursor (Game|GetPlayerController 0) true)
    (Game|SetGamePaused true)
    (else
      (Variables|Default|SetIsPauseMenuOpened? false)
      (Widget|RemovefromParent (Variables|Default|GetPauseMenuWidget))
      (Game|SetGamePaused false)
      (Input|SetInputModeGameOnly (Game|GetPlayerController 0) false)
      (Variables|/Script/Engine.PlayerController|SetbShowMouseCursor (Game|GetPlayerController 0) false))))

(event EventBeginPlay
  (bind _returnvalue (Game|GetPlayerController 0))
  (Input|SetInputModeGameOnly _returnvalue false)
  (Variables|/Script/Engine.PlayerController|SetbShowMouseCursor _returnvalue true))

(event Input|KeyboardEvents|1
  (params (Key :type Key%20Structure :default "None"))
  (:Pressed
    (bind _asbp_game_instance (Utilities|Casting|CastToBP_GameInstance (Game|GetGameInstance)))
    (Default|AddMoney _asbp_game_instance 10)))

(event Input|KeyboardEvents|2
  (params (Key :type Key%20Structure :default "None"))
  (:Pressed
    (bind _asbp_game_instance (Utilities|Casting|CastToBP_GameInstance (Game|GetGameInstance)))
    (Default|RemoveMoney _asbp_game_instance 10)))

(fn ConstructionScript)